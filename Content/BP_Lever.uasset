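; BP_Lever is an interactable lever that flips a flag, with prompt text for opening or closing a door.
; Interact calls FlipFlag on the game mode's FlagManager component with the lever's Flag, then toggles its own IsEnable.
; GetDescription picks "Close door" or "Open door" from that local boolean rather than querying the manager.
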(event EventInteract
  (Class|FlagManager|FlipFlag (Actor|GetComponentbyClass (Game|GetGameMode) "/Script/IntroductionUnreal.FlagManager") (Variables|Default|GetFlag))
  (Variables|Default|SetIsEnable (not (Variables|Default|GetIsEnable))))

(fn ConstructionScript)

(fn GetDescription
  (return (Utilities|String|SelectString "Close door" "Open door" (Variables|Default|GetIsEnable))))