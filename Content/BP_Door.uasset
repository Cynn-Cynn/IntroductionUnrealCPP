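; Interactable sliding door that toggles between closed and open, with an Open/Close prompt that is blank while it moves or cannot be opened.
; Interact checks CanOpenDoor, then DoorInteraction plays or reverses the MoveDoor timeline, lerping DoorPivot by MovementOffset and flipping IsOpen when finished.
; FlagTrigger bindings for automatic opening, such as by a lever, are unconnected, and CanOpenDoor's flag check is unused.
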(event Custom|DoorInteraction
  (if (not (Variables|Default|GetIsMoving))
    (Variables|Default|SetIsMoving true)
    (if (Variables|Default|GetIsOpen)
      (bind _movement (Timeline|MoveDoor Reverse)
        (:Update
          (Transformation|SetRelativeLocation (Variables|Default|GetDoorPivot) (Math|Vector|Lerp(Vector) "0, 0, 0" (Variables|Default|GetMovementOffset) _movement) false false))
        (:Finished
          (Variables|Default|SetIsOpen (not (Variables|Default|GetIsOpen)))
          (Variables|Default|SetIsMoving false)))
      (else
        (Timeline|MoveDoor Play)))))

(event EventBeginPlay
  ;[0.15 0.15 0.15 0.5] Setup pour se brancher a un event automatique, par exemple pour se lier à un levier
)

(event EventDestroyed
  ;[0.15 0.15 0.15 0.5] Setup pour se brancher a un event automatique, par exemple pour se lier à un levier
)

(event EventInteract
  (if (Utilities|CanOpenDoor)
    (CallFunction|DoorInteraction)))

(fn ConstructionScript)

(fn GetDescription
  (return (Utilities|String|SelectString "" (Utilities|String|SelectString "Close" "Open" (Variables|Default|GetIsOpen)) (or (Variables|Default|GetIsMoving) (not (Utilities|CanOpenDoor))))))