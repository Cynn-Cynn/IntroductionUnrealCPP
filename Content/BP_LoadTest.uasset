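; BP_LoadTest is a test actor that changes its sphere's material according to the Level.Test flag.
; On BeginPlay it binds ChangeColor to its FlagTrigger's OnFlagValid event.
; ChangeColor reads the flag from the FlagManager component on the game mode and applies one of two materials for values 0 and 1.
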(event Custom|ChangeColor
  (bind _returnvalue (Game|GetGameMode))
  (bind _sphere (Variables|Default|GetSphere))
  (bind _returnvalue_2 (Actor|GetComponentbyClass _returnvalue "/Script/IntroductionUnreal.FlagManager"))
  (Utilities|IsValid _returnvalue_2
    (:Is%20Valid
      (switch int (Class|FlagManager|GetFlagValue _returnvalue_2 "(TagName=\"Level.Test\")")
        (:0
          (Rendering|Material|SetMaterial _sphere 0 "/DatasmithContent/Materials/AliasReference.AliasReference"))
        (:1
          (Rendering|Material|SetMaterial _sphere 0 "/Engine/BasicShapes/BasicShapeMaterial.BasicShapeMaterial"))))))

(event EventBeginPlay
  (EventDispatchers|BindEventtoOnFlagValid (Variables|Default|GetFlagTrigger) (delegate Custom|ChangeColor)))

(fn ConstructionScript)